(event `self.ReceiveBeginPlay`
  (bind _returnvalue (`GameplayStatics.GetActorOfClass` "/Game/StealthGame/Core/Characters/PlayerCharacter/BP_ThirdPersonCharacterCustom.BP_ThirdPersonCharacterCustom_C")))

(event `self.Box collision.OnComponentBeginOverlap`
  (params (OverlappedComponent :type "PrimitiveComponent Object Reference") (OtherActor :type "Actor Object Reference") (OtherComp :type "PrimitiveComponent Object Reference") (OtherBodyIndex :type Integer) (bFromSweep :type Boolean) (SweepResult :type "HitResult Structure (by ref)"))
  (bind _asbp_enemy_companion (cast `/Game/BP_EnemyCompanion` OtherActor)
    (:`then`
      (`self.K2_DestroyActor` _asbp_enemy_companion)
      (bind _result (`/Engine/EditorBlueprintResources/StandardMacros.IncrementFloat` (`KismetMathLibrary.Conv_IntToDouble` (`self.CactusCounter`)))
        (:`  `
          (set `self.CactusCounter` (`KismetMathLibrary.FTrunc` _result))
          (if (>= (`self.CactusCounter`) 2)
            (`/Game/StealthGame/Core/Characters/PlayerCharacter/BP_ThirdPersonCharacterCustom.You Win` (stale `self.ReceiveBeginPlay` _returnvalue))
            (else
              (`KismetSystemLibrary.PrintString` "Thank you! You're a Hero!"))))))
    (:`CastFailed`
      (`KismetSystemLibrary.PrintString` "Not A Cactus"))))

(fn `UserConstructionScript`)