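; BP_LevelMusic handles level music in the stealth game through two audio components, MusicAudio1 and MusicAudio2.
; On BeginPlay it calls a fade-out on MusicAudio1 and lowers its volume multiplier.
; When MusicAudio1 reports that it has finished, MusicAudio2 fades in at the same reduced volume, handing off from the first track to the second.
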(event `self.ReceiveBeginPlay`
  (set `self.MusicAudio1` null)
  (`AudioComponent.FadeOut` (`self.MusicAudio1`) 2.0 0.0 "Linear")
  (`AudioComponent.SetVolumeMultiplier` (`self.MusicAudio1`) 0.3))

(event `self.MusicAudio1.OnAudioFinished`
  (set `self.MusicAudio2` null)
  (`AudioComponent.FadeIn` (`self.MusicAudio2`) 2.0 1.0 0.0 "Linear")
  (`AudioComponent.SetVolumeMultiplier` (`self.MusicAudio2`) 0.3))

(fn `UserConstructionScript`)